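; BeeSwarmTarget_BP is a player-steered pawn that acts as the target for a swarm of bees.
; Horizontal and vertical axis inputs move it along world X and Z.
; On BeginPlay it spawns SwarmSize Bee_BP actors at its own transform, regardless of collision, and sets itself as each bee's BeeSwarmTarget.
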(event EventBeginPlay
  (for _index (range 0 (Variables|Default|GetSwarmSize))
    (Utilities|FlowControl|Sequence
      (:then_0
        (bind _returnvalue (Game|SpawnActorfromClass "/Game/Bee_BP.Bee_BP_C" (Transformation|GetActorTransform) "AlwaysSpawn" 0 0))
        (Variables|/Game/Bee_BP.Bee_BP_C|SetBeeSwarmTarget _returnvalue self)))))

(event Input|AxisEvents|InputAxisHorizontal_Axis
  (params (AxisValue :type Float%20%28single-precision%29))
  (Pawn|Input|AddMovementInput "1.000000, 0, 0" AxisValue false))

(event Input|AxisEvents|InputAxisVertical_Axis
  (params (AxisValue :type Float%20%28single-precision%29))
  (Pawn|Input|AddMovementInput "0.000000,0.000000,1.000000" AxisValue false))

(fn ConstructionScript)