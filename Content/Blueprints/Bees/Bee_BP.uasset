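; Bee actor that chases a BeeSwarmTarget as a physics-driven 2D Paper flipbook sprite.
; Each tick it accelerates BeeBall toward the target beyond a small dead zone, adding braking and sideways damping when not moving fast enough toward it.
; The ball's rotation is reset, while the sprite flips on horizontal velocity with a threshold against flicker.
; A buzz offset jitters the sprite, its direction randomly rotated in the XZ plane on a tick counter.
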(event EventTick
  (params (DeltaSeconds :type Float%20%28single-precision%29))
  (bind _returnvalue (Transformation|GetActorLocation))
  (bind _beeswarmtarget (Variables|Default|GetBeeSwarmTarget))
  (bind _paperflipbook (Variables|Default|GetPaperFlipbook))
  (bind _beeball (Variables|Default|GetBeeBall))
  (bind _returnvalue_2 (Transformation|GetActorLocation _beeswarmtarget))
  (bind _returnvalue_3 (- _returnvalue_2 _returnvalue))
  (bind _returnvalue_4 (Math|Vector|Normalize _returnvalue_3))
  (bind _returnvalue_5 (Math|Vector|CrossProduct "0,1.000000, 0" _returnvalue_4))
  (Utilities|FlowControl|Sequence
    (:then_0
      ;[1 1 1] Heading Towards
      (bind _returnvalue_6 (Physics|GetPhysicsLinearVelocity (Variables|Default|GetBeeBall) "None")))
    (:then_1
      ;[1 1 1] If Distance >
      (if (> (Math|Vector|VectorLength _returnvalue_3) 2e+01)
        ;[1 1 1] If Heading Towards
        (if (> (Math|Vector|DotProduct _returnvalue_4 _returnvalue_6) 1e+01)
          ;[1 1 1] Accelerato
          (Physics|AddForce (Variables|Default|GetBeeBall) (* _returnvalue_4 1.5e+03) "None" true :!label _label)
          (else
            (Utilities|FlowControl|Sequence
              (:then_0
                (goto _label))
              (:then_1
                ;[1 1 1] Rallentato
                (bind _returnvalue_7 (Physics|GetPhysicsLinearVelocity _beeball "None"))
                (Physics|AddForce _beeball (* _returnvalue_7 -1 1e+01) "None" true))
              (:then_2
                ;[1 1 1] Sideways Velocity Damp
                (Physics|AddForce (Variables|Default|GetBeeBall) (* _returnvalue_5 -1 (Math|Vector|DotProduct _returnvalue_5 _returnvalue_7) 2e+01 (Variables|Default|GetSidewaysSnapMultiplier)) "None" true)))))))
    (:then_2
      ;[1 1 1] Flip or No Flip
      (bind _returnvalue_8 (Physics|GetPhysicsLinearVelocity (Variables|Default|GetBeeBall) "None"))
      (Utilities|FlowControl|Sequence
        (:then_0
          (if (> (.X (Math|Vector|BreakVector _returnvalue_8)) 2e+02)
            (Variables|Default|SetFlipped false)))
        (:then_1
          (if (< (.X (Math|Vector|BreakVector _returnvalue_8)) -2e+02)
            (Variables|Default|SetFlipped true)))))
    (:then_3
      ;[1 1 1] Rotating
      (Utilities|FlowControl|Sequence
        (:then_0
          (Transformation|SetRelativeRotation (Variables|Default|GetBeeBall) "0, 0, 0" false false))
        (:then_1
          (if (Variables|Default|GetFlipped)
            (Transformation|SetRelativeRotation _paperflipbook "0,180.000000, 0" false false)
            (else
              (Transformation|SetRelativeRotation _paperflipbook "0, 0, 0" false false))))))
    (:then_4
      ;[1 1 1] Buzzing
      (Transformation|SetRelativeLocation (Variables|Default|GetPaperFlipbook) (* (Variables|Default|GetBuzzDirection) 2.0 (Variables|Default|GetBuzzMultiplier)) false false))
    (:then_5
      ;[1 1 1] Buzz Timer
      (bind _output_get (Variables|Default|SetBuzzCounter (Class|KismetMathLibrary|Wrap (+ (Variables|Default|GetBuzzCounter) 1) 0 (Variables|Default|GetBuzzWaitTicks))))
      (if (== _output_get (Variables|Default|GetBuzzWaitTicks))
        ;[1 1 1] Buzz Wait Ticks
        (Variables|Default|SetBuzzDirection (Math|Vector|Normalize (Math|Vector|RotateVectorAroundAxis (Variables|Default|GetBuzzDirection) (Math|Random|RandomFloatinRange 0.0 1.8e+02) "0,1.000000,0.000000")))))))

(fn ConstructionScript)