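; Bee actor that steers a physics-driven BeeBall toward a BeeSwarmTarget actor.
; Each tick, beyond a small distance, it applies a mass-independent force toward the target, adding velocity-opposing braking when not already moving toward it fast enough.
; The ball's relative rotation is reset every tick to keep it from rolling.
; A sideways damping force is present but unconnected, so it never runs.
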(event EventTick
  (params (DeltaSeconds :type Float%20%28single-precision%29))
  (bind _returnvalue (Transformation|GetActorLocation))
  (bind _beeswarmtarget (Variables|Default|GetBeeSwarmTarget))
  (bind _beeball (Variables|Default|GetBeeBall))
  (bind _returnvalue_2 (Transformation|GetActorLocation _beeswarmtarget))
  (bind _returnvalue_3 (- _returnvalue_2 _returnvalue))
  (bind _returnvalue_4 (Math|Vector|Normalize _returnvalue_3))
  (Utilities|FlowControl|Sequence
    (:then_0
      ;[1 1 1] Heading Towards
      (bind _returnvalue_5 (Physics|GetPhysicsLinearVelocity (Variables|Default|GetBeeBall) "None")))
    (:then_1
      (if (> (Math|Vector|VectorLength _returnvalue_3) 2e+01)
        (if (> (Math|Vector|DotProduct _returnvalue_4 _returnvalue_5) 1e+01)
          ;[1 1 1] Accelerato
          (Physics|AddForce (Variables|Default|GetBeeBall) (* _returnvalue_4 1.5e+03) "None" true :!label _label)
          (else
            (Utilities|FlowControl|Sequence
              (:then_0
                (goto _label))
              (:then_1
                ;[1 1 1] Rallentato
                (bind _returnvalue_6 (Physics|GetPhysicsLinearVelocity _beeball "None"))
                (Physics|AddForce _beeball (* _returnvalue_6 -1 1e+01) "None" true)))))))
    (:then_2
      (Transformation|SetRelativeRotation (Variables|Default|GetBeeBall) "0, 0, 0" false false))))

(fn ConstructionScript)